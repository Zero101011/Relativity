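; Interactable button actor that plays an assigned level sequence when the player presses Action inside its overlap area.
; Overlap shows a text prompt and a custom-depth highlight on the cube, colored through a stencil code.
; Each press alternates forward and reverse playback via a flag flipped when the sequence finishes.
; The GravityCharacter's walk speed is zeroed during playback, then restored to the value cached at BeginPlay.
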(event Custom|FreezePlayer
  (bind _asgravity_character (Utilities|Casting|CastToGravityCharacter (Game|Player|GetPlayerPawn 0)))
  (Variables|/Script/Engine.CharacterMovementComponent|SetMaxWalkSpeed (Variables|/Script/Engine.Character|GetCharacterMovement _asgravity_character) 0.0))

(event Custom|UnfreezePlayer
  (bind _asgravity_character (Utilities|Casting|CastToGravityCharacter (Game|Player|GetPlayerPawn 0)))
  (Variables|/Script/Engine.CharacterMovementComponent|SetMaxWalkSpeed (Variables|/Script/Engine.Character|GetCharacterMovement _asgravity_character) (Variables|Default|GetMoveSpeed)))

(event Custom|ButtonPressed
  (bind _sequence (Variables|Default|GetSequence))
  (bind _sequenceplayer (Variables|/Script/LevelSequence.LevelSequenceActor|GetSequencePlayer _sequence))
  ;[1 1 1] When player presses F check if they are in the trigger volume and if anim is complete, depending on if anim is complete either play or reverse anim.
  (if (Variables|Default|GetPlayerOverlap)
    (if (Variables|Default|GetDoReverse?)
      (Class|MovieSceneSequencePlayer|PlayReverse _sequenceplayer)
      (else
        (Sequencer|Player|Play _sequenceplayer :!class /Script/MovieScene.MovieSceneSequencePlayer)))
    (CallFunction|FreezePlayer)
    (EventDispatchers|BindEventtoOnFinished _sequenceplayer (delegate Custom|Onfinished))))

(event Custom|Onfinished
  ;[1 1 1] When player presses F check if they are in the trigger volume and if anim is complete, depending on if anim is complete either play or reverse anim.
  (CallFunction|UnfreezePlayer)
  (if (Variables|Default|GetDoReverse?)
    (Variables|Default|SetDoReverse? false)
    (else
      (Variables|Default|SetDoReverse? true)))
  (Sequencer|Player|Pause (Variables|/Script/LevelSequence.LevelSequenceActor|GetSequencePlayer (Variables|Default|GetSequence))))

(event Collision|EventActorBeginOverlap
  (params (OtherActor :type Actor%20Object%20Reference))
  ;[1 1 1] Set visibility for on screen advice & set player overlap bool
  (bind _output_get (Variables|Default|SetPlayerOverlap (== OtherActor (Game|Player|GetPlayerPawn 0))))
  (if _output_get
    (Rendering|SetVisibility (Variables|Default|GetText) true false)
    (Rendering|SetRenderCustomDepth (Variables|Default|GetCube) true)))

(event Collision|EventActorEndOverlap
  (params (OtherActor :type Actor%20Object%20Reference))
  ;[1 1 1] Set visibility for on screen advice & set player overlap bool
  (Variables|Default|SetPlayerOverlap false)
  (if (== OtherActor (Game|Player|GetPlayerPawn 0))
    (Rendering|SetVisibility (Variables|Default|GetText) false false)
    (Rendering|SetRenderCustomDepth (Variables|Default|GetCube) false)))

(event EventBeginPlay
  ;[1 1 1] Enable Player Input & Set base speed for animation reset
  (Rendering|SetCustomDepthStencilValue (Variables|Default|GetCube) (Variables|Default|GetItemColorCode))
  (Input|EnableInput (Game|GetPlayerController 0))
  (bind _asgravity_character (Utilities|Casting|CastToGravityCharacter (Game|Player|GetPlayerPawn 0)))
  (Variables|Default|SetMoveSpeed (Variables|/Script/Engine.CharacterMovementComponent|GetMaxWalkSpeed (Variables|/Script/Engine.Character|GetCharacterMovement _asgravity_character))))

(event Input|ActionEvents|InputActionAction
  (params (Key :type Key%20Structure))
  ;[1 1 1] When player presses F check if they are in the trigger volume and if anim is complete, depending on if anim is complete either play or reverse anim.
  (:Pressed
    (CallFunction|ButtonPressed)))

(fn ConstructionScript)