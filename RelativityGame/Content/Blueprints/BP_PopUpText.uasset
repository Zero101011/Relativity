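; BP_PopUpText is an actor that pops up custom text while the player pawn overlaps it.
; On BeginPlay it writes CustomText into its TextRender component and toggles that component's visibility.
; Begin and end overlap events from player pawn 0 each toggle visibility again, so the result depends on the component's initial state rather than an explicit show or hide.
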(event Collision|EventActorBeginOverlap
  (params (OtherActor :type Actor%20Object%20Reference))
  (if (== OtherActor (Game|Player|GetPlayerPawn 0))
    (Rendering|ToggleVisibility (Variables|Default|GetTextRender) false)))

(event Collision|EventActorEndOverlap
  (params (OtherActor :type Actor%20Object%20Reference))
  (if (== OtherActor (Game|Player|GetPlayerPawn 0))
    (Rendering|ToggleVisibility (Variables|Default|GetTextRender) false)))

(event EventBeginPlay
  (bind _textrender (Variables|Default|GetTextRender))
  (Rendering|Components|TextRender|SetText _textrender (Variables|Default|GetCustomText))
  (Rendering|ToggleVisibility _textrender false))

(fn ConstructionScript)